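; BP_SameDoor is a room exit door that, when opened, spawns the next BP_Room at the current room's difficulty.
; OpenEvent increments the game instance's room count, flags the new room as the finish at MaxRooms, offsets it by its entrance position and fills it.
; It then updates the current and previous rooms, disables its box collision, has the previous room replace its harder door, and swings open via a Timeline.
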(event `Open Event`
  (bind _asbp_game_instance (cast `/Game/BluePrints/BP_GameInstance` (`GameplayStatics.GetGameInstance`) :!pure true))
  (bind _asbp_game_instance_2 (cast `/Game/BluePrints/BP_GameInstance` (`GameplayStatics.GetGameInstance`) :!pure true))
  (`/Engine/EditorBlueprintResources/StandardMacros.IncrementInt` (`/Game/BluePrints/BP_GameInstance.Rooms` _asbp_game_instance)
    (:`  `
      (set `self.Difficulty` (`/Game/BluePrints/BP_Room.Difficulty` (`/Game/BluePrints/BP_GameInstance.Current Room` _asbp_game_instance)))
      (bind _returnvalue (`|SpawnActorFromClass` "/Game/BluePrints/BP_Room.BP_Room_C" (`self.GetTransform`) "Undefined" "MultiplyWithRoot" null (`self.Difficulty`) (== (`/Game/BluePrints/BP_GameInstance.Rooms` _asbp_game_instance) (`/Game/BluePrints/BP_GameInstance.Max Rooms` _asbp_game_instance)) null))
      (`self.K2_SetActorLocation` _returnvalue (+ (`self.K2_GetActorLocation` _returnvalue) (`KismetMathLibrary.MakeVector` 0.0 (* (`/Game/BluePrints/BP_Room.EntranceX` _returnvalue) -400))) false false)
      (`/Game/BluePrints/BP_Room.Fill Event` _returnvalue)
      (set `/Game/BluePrints/BP_GameInstance.Previous Room` (`/Game/BluePrints/BP_GameInstance.Current Room` _asbp_game_instance_2) _asbp_game_instance_2)
      (set `/Game/BluePrints/BP_GameInstance.Current Room` _returnvalue _asbp_game_instance_2)
      (`PrimitiveComponent.SetCollisionEnabled` (`self.Box`) "NoCollision")
      (`/Game/BluePrints/BP_Room.Replace Harder Door` (`/Game/BluePrints/BP_GameInstance.Previous Room` (cast `/Game/BluePrints/BP_GameInstance` (`GameplayStatics.GetGameInstance`) :!pure true)))
      (bind (_direction _doorfloat) (`Timeline|Timeline` :!via `PlayFromStart`)
        (:`Update`
          (`SceneComponent.K2_SetRelativeRotation` (`self.Door`) (`KismetMathLibrary.MakeRotator` 0.0 0.0 (`KismetMathLibrary.Lerp` 90.0 180.0 _doorfloat)) false false))))))

(fn `UserConstructionScript`)