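; BP_PlayerState tracks the player's HP and handles player death.
; ChangeHP adds a signed change to HP, prints the new value, then calls CheckForDeath to test whether HP is zero or below.
; On death, DeathEvent destroys the character at player index 0, regardless of which player the state belongs to, and prints a death message; no respawn logic is present.
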(event `Death Event`
  (`self.K2_DestroyActor` (`GameplayStatics.GetPlayerCharacter` 0))
  (`KismetSystemLibrary.PrintString` "you died"))

(fn `ChangeHP`
  (params (change :type Integer))
  (set `self.HP` (+ change (`self.HP`)))
  (`KismetSystemLibrary.PrintString` (`KismetStringLibrary.Conv_IntToString` (`self.HP`)))
  (bind _death (`self.CheckForDeath`))
  (if _death
    (`self.Death Event`)))

(fn `CheckForDeath`
  (returns (Death :type Boolean))
  (return (<= (`self.HP`) 0)))

(fn `UserConstructionScript`)