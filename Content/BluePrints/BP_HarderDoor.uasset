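; BP_HarderDoor is a door that, when opened, spawns the next procedural room one difficulty level above the current one, or at zero before the game starts.
; It increments the GameInstance room count, flags the room as finish at the maximum, offsets it by its entrance and calls its fill event.
; It then updates current and previous rooms, disables box collision, replaces the previous room's matching door once started, and swings open via timeline.
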(event `Open Door`
  (bind _asbp_game_instance (cast `/Game/BluePrints/BP_GameInstance` (`GameplayStatics.GetGameInstance`) :!pure true))
  (bind _asbp_game_instance_2 (cast `/Game/BluePrints/BP_GameInstance` (`GameplayStatics.GetGameInstance`) :!pure true))
  (bind _asbp_game_instance_3 (cast `/Game/BluePrints/BP_GameInstance` (`GameplayStatics.GetGameInstance`) :!pure true))
  (`/Engine/EditorBlueprintResources/StandardMacros.IncrementInt` (`/Game/BluePrints/BP_GameInstance.Rooms` _asbp_game_instance_2)
    (:`  `
      (if (`/Game/BluePrints/BP_GameInstance.Started` _asbp_game_instance_2)
        (set `self.Difficulty` (+ (`/Game/BluePrints/BP_Room.Difficulty` (`/Game/BluePrints/BP_GameInstance.Current Room` _asbp_game_instance_2)) 1))
        (else
          (set `self.Difficulty` 0)))
      (bind _returnvalue (`|SpawnActorFromClass` "/Game/BluePrints/BP_Room.BP_Room_C" (`self.GetTransform`) "Undefined" "MultiplyWithRoot" null (`self.Difficulty`) (== (`/Game/BluePrints/BP_GameInstance.Rooms` _asbp_game_instance_2) (`/Game/BluePrints/BP_GameInstance.Max Rooms` _asbp_game_instance_2)) null))
      (`self.K2_SetActorLocation` _returnvalue (+ (`self.K2_GetActorLocation` _returnvalue) (`KismetMathLibrary.MakeVector` 0.0 (* (`/Game/BluePrints/BP_Room.EntranceX` _returnvalue) -400))) false false)
      (`/Game/BluePrints/BP_Room.Fill Event` _returnvalue)
      (set `/Game/BluePrints/BP_GameInstance.Previous Room` (`/Game/BluePrints/BP_GameInstance.Current Room` _asbp_game_instance_3) _asbp_game_instance_3)
      (set `/Game/BluePrints/BP_GameInstance.Current Room` _returnvalue _asbp_game_instance_3)
      (`PrimitiveComponent.SetCollisionEnabled` (`self.Box`) "NoCollision")
      (if (`/Game/BluePrints/BP_GameInstance.Started` _asbp_game_instance)
        (`/Game/BluePrints/BP_Room.Replace Same Door` (`/Game/BluePrints/BP_GameInstance.Previous Room` _asbp_game_instance))
        (bind (_direction _doorfloat) (`Timeline|OpenDoor Timeline` :!via `PlayFromStart` :!label _label)
          (:`Update`
            (`SceneComponent.K2_SetRelativeRotation` (`self.Door`) (`KismetMathLibrary.MakeRotator` 0.0 0.0 (`KismetMathLibrary.Lerp` 90.0 180.0 _doorfloat)) false false)))
        (else
          (goto _label :!via `PlayFromStart`))))))

(fn `UserConstructionScript`)