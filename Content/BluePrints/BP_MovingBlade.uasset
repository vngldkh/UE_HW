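; BP_MovingBlade is an actor that slides a child rotating blade between two points.
; On BeginPlay it derives the end point from its start location, rotation axes and MoveVector, then plays a timeline that lerps the actor's position without sweep.
; MoveSpeed drives both the timeline play rate and the child BP_RotatingBlade's rotation speed.
; SetSpeed updates both at once and returns the actor itself.
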(event `self.ReceiveBeginPlay`
  (bind _returnvalue (`self.K2_GetActorLocation`))
  (bind _movevector (`self.moveVector`))
  (bind (_x _y) (`KismetMathLibrary.GetAxes` (`self.K2_GetActorRotation`)))
  (set `self.startPoint` _returnvalue)
  (set `self.endPoint` (+ _returnvalue (+ (* _x _movevector) (* _y _movevector))))
  (`self.Update Speed`)
  (`self.MoveEvent`))

(event `MoveEvent`
  (bind (_direction _move) (`Timeline|Move Timeline` :!via `PlayFromStart`)
    (:`Update`
      (`self.K2_SetActorLocation` (`KismetMathLibrary.VLerp` (`self.startPoint`) (`self.endPoint`) _move)))))

(event `Update Speed`
  (bind _asbp_rotating_blade (cast `/Game/BluePrints/BP_RotatingBlade` (`ChildActorComponent.ChildActor` (`self.Blade`)) :!pure true))
  (set `/Game/BluePrints/BP_RotatingBlade.rotation_speed` (`self.move_speed`) _asbp_rotating_blade)
  (`/Game/BluePrints/BP_RotatingBlade.Set Speed` _asbp_rotating_blade)
  (`TimelineComponent.SetPlayRate` (`self.Move Timeline`) (`self.move_speed`)))

(fn `SetSpeed`
  (params (Speed :type "Float (double-precision)"))
  (returns (Actor :type "/Game/BluePrints/BP_MovingBlade Object Reference"))
  (set `self.move_speed` Speed)
  (`self.Update Speed`)
  (return self))

(fn `UserConstructionScript`)