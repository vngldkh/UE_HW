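; BP_Room is a procedurally generated trap room, sized and populated from the DT_Room_Difficulties row selected by Difficulty.
; The construction script builds instanced floor and walls, leaving random gaps for one entrance and two exits (same and harder).
; BeginPlay shuffles trap and plain tiles, inserting plain entries intended for the openings.
; Each trap tile spawns a random blade, spike, spike wall or fire actor, aligned to the room's rotation.
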(event `self.ReceiveBeginPlay`
  (bind _newparam (`self.Generate Content Array`))
  (`self.Fill Room` _newparam))

(fn `Fill Room`
  (params (Objects :type "Array of /Game/Data/E_TileTypes Enum"))
  (for (_array_element _array_index) Objects
    (bind (_x _y) (`self.Get XY` _array_index))
    (`self.Fill Tile` _x _y _array_element)))

(fn `Fill Tile`
  (params (X :type Integer) (Y :type Integer) (TileType :type "/Game/Data/E_TileTypes Enum" :default "NewEnumerator1"))
  (switch `/Game/Data/E_TileTypes` TileType
    (:`NewEnumerator0`
      (bind _trap_ref (`self.Place Trap` X Y (cast `/Game/Data/E_TrapTypes` (`KismetMathLibrary.Conv_IntToByte` (`KismetMathLibrary.RandomInteger` 4)))))
      (`KismetArrayLibrary.Array_Add` (`self.Actors`) _trap_ref))))

(fn `Generate Content Array`
  (returns (NewParam :type "Array of /Game/Data/E_TileTypes Enum"))
  (locals (Objects :type "Array of /Game/Data/E_TileTypes Enum") (`Plain Count` :type Integer))
  (set `local.Plain Count` (- (* (`self.MaxX`) (`self.MaxY`)) 3))
  (for _ (range (`.TrapsCount_20_320917734474D400FD6943B6968A95B7` (break `/Game/Data/S_RoomInfo` (`self.Content`))))
    (`KismetArrayLibrary.Array_Add` (`local.Objects`) "NewEnumerator0")
    (`/Engine/EditorBlueprintResources/StandardMacros.DecrementInt` (`local.Plain Count`)))
  (for _ (range (`local.Plain Count`))
    (`KismetArrayLibrary.Array_Add` (`local.Objects`) "NewEnumerator1"))
  (`KismetArrayLibrary.Array_Shuffle` (`local.Objects`))
  (`KismetArrayLibrary.Array_Insert` (`local.Objects`) "NewEnumerator1" (`self.EntranceX`))
  (`KismetArrayLibrary.Array_Insert` (`local.Objects`) "NewEnumerator1" (+ (`self.SameExitX`) (* (`self.MaxX`) (- (`self.MaxY`) 1))))
  (`KismetArrayLibrary.Array_Insert` (`local.Objects`) "NewEnumerator1" (+ (`self.HarderExitX`) (* (`self.MaxX`) (- (`self.MaxY`) 1))))
  (return (`local.Objects`)))

(fn `Get Absolute XYZ`
  (params (`Tile X` :type Integer) (`Tile Y` :type Integer))
  (returns (`Tile Coords` :type "Vector Structure"))
  (locals (Offset :type "Vector Structure"))
  (bind _tilesize (`self.TileSize`))
  (bind _offset (`local.Offset`))
  (bind (_x _y) (`KismetMathLibrary.GetAxes` (`self.K2_GetActorRotation`)))
  (set `local.Offset` (`KismetMathLibrary.MakeVector` (`KismetMathLibrary.Conv_IntToDouble` (* `Tile X` _tilesize)) (`KismetMathLibrary.Conv_IntToDouble` (* `Tile Y` _tilesize))))
  (return (+ (+ (* _x _offset) (* _y _offset)) (`self.K2_GetActorLocation`))))

(fn `Get XY`
  (params (i :type Integer))
  (returns (X :type Integer) (Y :type Integer))
  (bind _maxy (`self.MaxY`))
  (return (/ i _maxy) (mod i _maxy)))

(fn `Import Room Info`
  (bind _outrownames (`DataTableFunctionLibrary.GetDataTableRowNames` "/Game/Data/DT_Room_Difficulties.DT_Room_Difficulties"))
  (bind _returnvalue (`|GetDataTableRow` "/Game/Data/DT_Room_Difficulties.DT_Room_Difficulties" (`|GetArrayItem` _outrownames (`self.Difficulty`)))
    (:`then`
      (set `self.Content` _returnvalue))))

(fn `Place Blade Trap`
  (params (`Tile Location` :type "Vector Structure"))
  (returns (`Trap ref` :type "Actor Object Reference"))
  (locals (Offset :type "Vector Structure" :default (50.0 50.0 0.0)))
  (bind _returnvalue (`self.K2_GetActorRotation`))
  (bind _offset (`local.Offset`))
  (bind (_x _y) (`KismetMathLibrary.GetAxes` _returnvalue))
  (bind _returnvalue_2 (`|SpawnActorFromClass` "/Game/BluePrints/BP_MovingBlade.BP_MovingBlade_C" (`KismetMathLibrary.MakeTransform` (+ `Tile Location` (+ (* _x _offset) (* _y _offset))) _returnvalue) "Undefined" "MultiplyWithRoot" null null))
  (return _returnvalue_2))

(fn `Place Fire Trap`
  (params (`Tile Location` :type "Vector Structure"))
  (returns (`Trap ref` :type "Actor Object Reference"))
  (locals (Offset :type "Vector Structure" :default (200.0 200.0 0.0)))
  (bind _returnvalue (`self.K2_GetActorRotation`))
  (bind _offset (`local.Offset`))
  (bind (_x _y) (`KismetMathLibrary.GetAxes` _returnvalue))
  (bind _returnvalue_2 (`|SpawnActorFromClass` "/Game/BluePrints/BP_FiredFloor.BP_FiredFloor_C" (`KismetMathLibrary.MakeTransform` (+ `Tile Location` (+ (* _x _offset) (* _y _offset))) _returnvalue) "Undefined" "MultiplyWithRoot" null null))
  (return _returnvalue_2))

(fn `Place Spike Trap`
  (params (`Tile Location` :type "Vector Structure"))
  (returns (`Trap ref` :type "Actor Object Reference"))
  (bind _returnvalue (`|SpawnActorFromClass` "/Game/BluePrints/BP_SpikeTrap.BP_SpikeTrap_C" (`KismetMathLibrary.MakeTransform` `Tile Location` (`self.K2_GetActorRotation`)) "Undefined" "MultiplyWithRoot" null null))
  (return _returnvalue))

(fn `Place Spiked Wall`
  (params (`Tile Location` :type "Vector Structure"))
  (returns (`Trap ref` :type "Actor Object Reference"))
  (locals (Offset :type "Vector Structure" :default (200.0 200.0 0.0)))
  (bind _returnvalue (`self.K2_GetActorRotation`))
  (bind _offset (`local.Offset`))
  (bind (_x _y) (`KismetMathLibrary.GetAxes` _returnvalue))
  (bind _returnvalue_2 (`|SpawnActorFromClass` "/Game/BluePrints/BP_SpikeWall.BP_SpikeWall_C" (`KismetMathLibrary.MakeTransform` (+ `Tile Location` (+ (0.0 0.0 60.0) (+ (* _x _offset) (* _y _offset)))) _returnvalue) "Undefined" "MultiplyWithRoot" null null))
  (return _returnvalue_2))

(fn `Place Trap`
  (params (Tile_X :type Integer) (Tile_Y :type Integer) (`Trap Type` :type "/Game/Data/E_TrapTypes Enum" :default "NewEnumerator0"))
  (returns (`Trap ref` :type "Actor Object Reference"))
  (locals (Location :type "Vector Structure"))
  (bind _tile_coords (`self.Get Absolute XYZ` Tile_X Tile_Y))
  (set `local.Location` _tile_coords)
  (switch `/Game/Data/E_TrapTypes` `Trap Type`
    (:`NewEnumerator0`
      (bind _trap_ref (`self.Place Blade Trap` (`local.Location`)))
      (return _trap_ref))
    (:`NewEnumerator1`
      (bind _trap_ref_2 (`self.Place Spike Trap` (`local.Location`)))
      (return _trap_ref_2))
    (:`NewEnumerator2`
      (bind _trap_ref_3 (`self.Place Spiked Wall` (`local.Location`)))
      (return _trap_ref_3))
    (:`NewEnumerator3`
      (bind _trap_ref_4 (`self.Place Fire Trap` (`local.Location`)))
      (return _trap_ref_4))))

(fn `UserConstructionScript`
  (locals (X_i :type Integer) (Y_i :type Integer) (TileLocation :type "Vector Structure"))
  (bind (_content_trapscount _content_buffscount _content_debuffscount _content_randomeffects _content_maxxtiles _content_maxytiles) (break `/Game/Data/S_RoomInfo` (`self.Content`)))
  (bind _x_i (`local.X_i`))
  (bind _tilesize (`self.TileSize`))
  (`self.Import Room Info`)
  (set `self.MaxX` _content_maxxtiles)
  (set `self.MaxY` _content_maxytiles)
  (set `self.EntranceX` (`KismetMathLibrary.RandomIntegerInRange` 0 (- (`self.MaxX`) 1)))
  (set `self.SameExitX` (`KismetMathLibrary.RandomIntegerInRange` 0 (- (`self.MaxX`) 1)))
  (set `self.HarderExitX` (`KismetMathLibrary.RandomIntegerInRange` 0 (- (`self.MaxX`) 1)))
  (while (== (`self.SameExitX`) (`self.HarderExitX`))
    (set `self.HarderExitX` (`KismetMathLibrary.RandomIntegerInRange` 0 (- (`self.MaxX`) 1))))
  (for _index (range (* (`self.MaxX`) (`self.MaxY`)))
    (bind (_x _y) (`self.Get XY` _index))
    (set `local.Y_i` _x)
    (set `local.X_i` _y)
    (set `local.TileLocation` (`KismetMathLibrary.MakeVector` (`KismetMathLibrary.Conv_IntToDouble` (* (`local.X_i`) _tilesize)) (`KismetMathLibrary.Conv_IntToDouble` (* _tilesize (`local.Y_i`)))))
    (`InstancedStaticMeshComponent.AddInstance` (`self.Floor`) (`KismetMathLibrary.Conv_VectorToTransform` (`local.TileLocation`)) false)
    (if (and (== 0 (`local.Y_i`)) (!= (`local.X_i`) (`self.EntranceX`)))
      (`InstancedStaticMeshComponent.AddInstance` (`self.Wall`) (`KismetMathLibrary.Conv_VectorToTransform` (`local.TileLocation`)) false))
    (if (== 0 (`local.X_i`))
      (`InstancedStaticMeshComponent.AddInstance` (`self.Wall`) (`KismetMathLibrary.MakeTransform` (`local.TileLocation`) (`KismetMathLibrary.MakeRotator` 0.0 0.0 90.0)) false))
    (if (== (`local.X_i`) (- (`self.MaxX`) 1))
      (`InstancedStaticMeshComponent.AddInstance` (`self.Wall`) (`KismetMathLibrary.MakeTransform` (+ (`local.TileLocation`) (`KismetMathLibrary.MakeVector` (`self.TileSize`))) (`KismetMathLibrary.MakeRotator` 0.0 0.0 90.0)) false))
    (if (and (== (`local.Y_i`) (- (`self.MaxY`) 1)) (and (!= (`self.SameExitX`) _x_i) (!= _x_i (`self.HarderExitX`))))
      (`InstancedStaticMeshComponent.AddInstance` (`self.Wall`) (`KismetMathLibrary.Conv_VectorToTransform` (+ (`local.TileLocation`) (`KismetMathLibrary.MakeVector` 0.0 (`self.TileSize`)))) false))))