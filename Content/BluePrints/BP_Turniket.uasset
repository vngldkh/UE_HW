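; BP_Turniket is a one-way checkpoint that seals the passage and removes the area left behind when its trigger is crossed.
; On Box overlap it adds a Wall instance at its local origin and disables the trigger's collision so it cannot fire again.
; It then reads BP_GameInstance, destroying PreviousRoom if Started is set, or otherwise destroying the Start actor and setting Started.
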(event `self.Box.OnComponentBeginOverlap`
  (params (OverlappedComponent :type "PrimitiveComponent Object Reference") (OtherActor :type "Actor Object Reference") (OtherComp :type "PrimitiveComponent Object Reference") (OtherBodyIndex :type Integer) (bFromSweep :type Boolean) (SweepResult :type "HitResult Structure (by ref)"))
  (bind _asbp_game_instance (cast `/Game/BluePrints/BP_GameInstance` (`GameplayStatics.GetGameInstance`) :!pure true))
  (`InstancedStaticMeshComponent.AddInstance` (`self.Wall`) (`KismetMathLibrary.Conv_VectorToTransform` (0.0 0.0 0.0)) false)
  (`PrimitiveComponent.SetCollisionEnabled` (`self.Box`) "NoCollision")
  (if (`/Game/BluePrints/BP_GameInstance.Started` _asbp_game_instance)
    (`/Game/BluePrints/BP_Room.Destroy` (`/Game/BluePrints/BP_GameInstance.Previous Room` _asbp_game_instance))
    (else
      (`self.K2_DestroyActor` (`/Game/BluePrints/BP_GameInstance.Start` _asbp_game_instance))
      (set `/Game/BluePrints/BP_GameInstance.Started` true _asbp_game_instance))))

(fn `UserConstructionScript`)