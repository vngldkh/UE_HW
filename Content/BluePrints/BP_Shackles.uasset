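; BP_Shackles is a spinning hazard actor that slows the player on contact.
; When its mesh overlaps a BP_ThirdPersonCharacter, it calls that character's SlowEvent and destroys itself.
; From BeginPlay, a timeline lerps the actor through a half turn, then restarts RotationEvent from the new rotation to keep it spinning.
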(event `self.ReceiveBeginPlay`
  (`self.Rotation Event`))

(event `self.StaticMesh.OnComponentBeginOverlap`
  (params (OverlappedComponent :type "PrimitiveComponent Object Reference") (OtherActor :type "Actor Object Reference") (OtherComp :type "PrimitiveComponent Object Reference") (OtherBodyIndex :type Integer) (bFromSweep :type Boolean) (SweepResult :type "HitResult Structure (by ref)"))
  (bind _asbp_third_person_character (cast `/Game/ThirdPerson/Blueprints/BP_ThirdPersonCharacter` OtherActor))
  (`/Game/ThirdPerson/Blueprints/BP_ThirdPersonCharacter.Slow Event` _asbp_third_person_character)
  (`self.K2_DestroyActor`))

(event `Rotation Event`
  (bind _returnvalue (`self.K2_GetActorRotation`))
  (set `self.startRot` _returnvalue)
  (set `self.endRot` (`KismetMathLibrary.ComposeRotators` _returnvalue (struct :`Yaw` 180.0)))
  (bind (_direction _rot_float) (`Timeline|Timeline` :!via `PlayFromStart`)
    (:`Update`
      (`self.K2_SetActorRotation` (`KismetMathLibrary.RLerp` (`self.startRot`) (`self.endRot`) _rot_float true)))
    (:`Finished`
      (`self.Rotation Event`))))

(fn `UserConstructionScript`)