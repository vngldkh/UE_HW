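; BP_SpikeTrap is a moving spike hazard that damages actors it overlaps.
; On BeginPlay it records its location and a point 80 units below, then loops a timeline that lerps the actor between them without sweep, restarting each time it finishes.
; On overlap it reads damage from the SpikeTrap row of DT_TrapParams and passes it as a negative HP change to BP_GameMode's ChangePlayerHP.
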(event `self.ReceiveBeginPlay`
  (bind _returnvalue (`self.K2_GetActorLocation`))
  (set `self.startPoint` _returnvalue)
  (set `self.endPoint` (- _returnvalue (0.0 0.0 80.0)))
  (`self.MoveEvent`))

(event `MoveEvent`
  (bind (_direction _newtrack_0) (`Timeline|MoveTimeline` :!via `PlayFromStart`)
    (:`Update`
      (`self.K2_SetActorLocation` (`KismetMathLibrary.VLerp` (`self.startPoint`) (`self.endPoint`) _newtrack_0)))
    (:`Finished`
      (`self.MoveEvent`))))

(event `self.ReceiveActorBeginOverlap`
  (params (OtherActor :type "Actor Object Reference"))
  (bind _asbp_game_mode (cast `/Game/BluePrints/BP_GameMode` (`GameplayStatics.GetGameMode`)))
  (bind _returnvalue (`|GetDataTableRow` "/Game/Data/DT_TrapParams.DT_TrapParams" "SpikeTrap")
    (:`then`
      (`/Game/BluePrints/BP_GameMode.ChangePlayerHP` _asbp_game_mode OtherActor (* (`.Damage_6_6E1794974EA3B19A8A3433946FCE3C5B` (break `/Game/Data/S_Trap` _returnvalue)) -1)))))

(fn `UserConstructionScript`)