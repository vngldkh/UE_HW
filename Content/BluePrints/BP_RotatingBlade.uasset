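; BP_RotatingBlade is a blade actor that rotates its Blade component in an endless loop.
; On BeginPlay it stores the blade's relative rotation and a target a half turn away, then calls RotationEvent.
; RotationEvent plays a timeline that lerps between the two rotators and calls itself on finish, so each cycle restarts from the original rotation.
; The file contains no overlap or damage logic.
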(event `self.ReceiveBeginPlay`
  (bind _relativerotation (`SceneComponent.RelativeRotation` (`self.Blade`)))
  (set `self.startRotator` _relativerotation)
  (set `self.endRotator` (`KismetMathLibrary.ComposeRotators` _relativerotation (struct :`Roll` 180.0)))
  (`self.Rotation Event`))

(event `Rotation Event`
  (bind (_direction _move) (`Timeline|Timeline` :!via `PlayFromStart`)
    (:`Update`
      (`SceneComponent.K2_SetRelativeRotation` (`self.Blade`) (`KismetMathLibrary.RLerp` (`self.startRotator`) (`self.endRotator`) _move) false false))
    (:`Finished`
      (`self.Rotation Event`))))

(fn `UserConstructionScript`)