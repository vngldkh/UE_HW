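; BP_Heal is a health pickup that changes the HP of the actor that overlaps its Heart component, then destroys itself.
; On BeginPlay, one timeline lerps it between its start location and a point slightly above.
; A second timeline rotates it by half turns, restarting from the current rotation on finish to spin continuously.
; The HP change comes from DT_Health's Heal row and is applied through BP_GameMode.
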(event `self.ReceiveBeginPlay`
  (bind _returnvalue (`self.K2_GetActorLocation`))
  (set `self.startMoving` _returnvalue)
  (set `self.endMoving` (+ _returnvalue (0.0 0.0 30.0)))
  (`self.Move Event`)
  (`self.Rotation Event`))

(event `Move Event`
  (bind (_direction _move_float) (`Timeline|Move Timeline` :!via `PlayFromStart`)
    (:`Update`
      (`self.K2_SetActorLocation` (`KismetMathLibrary.VLerp` (`self.startMoving`) (`self.endMoving`) _move_float)))))

(event `Rotation Event`
  (bind _returnvalue (`self.K2_GetActorRotation`))
  (set `self.startRot` _returnvalue)
  (set `self.endRot` (`KismetMathLibrary.ComposeRotators` _returnvalue (struct :`Yaw` 180.0)))
  (bind (_direction _rot_float) (`Timeline|Rot Timeline` :!via `PlayFromStart`)
    (:`Update`
      (`self.K2_SetActorRotation` (`KismetMathLibrary.RLerp` (`self.startRot`) (`self.endRot`) _rot_float true)))
    (:`Finished`
      (`self.Rotation Event`))))

(event `self.Heart.OnComponentBeginOverlap`
  (params (OverlappedComponent :type "PrimitiveComponent Object Reference") (OtherActor :type "Actor Object Reference") (OtherComp :type "PrimitiveComponent Object Reference") (OtherBodyIndex :type Integer) (bFromSweep :type Boolean) (SweepResult :type "HitResult Structure (by ref)"))
  (bind _returnvalue (`|GetDataTableRow` "/Game/Data/DT_Health.DT_Health" "Heal")
    (:`then`
      (`/Game/BluePrints/BP_GameMode.ChangePlayerHP` (cast `/Game/BluePrints/BP_GameMode` (`GameplayStatics.GetGameMode`) :!pure true) OtherActor (`.Change_7_6E1794974EA3B19A8A3433946FCE3C5B` (break `/Game/Data/S_Health` _returnvalue)))
      (`self.K2_DestroyActor`))))

(fn `UserConstructionScript`)